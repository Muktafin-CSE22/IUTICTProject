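; BP_Mystery is a trigger actor that opens a one-time dialogue screen, UI_DiaWife2, apparently for the mysterious woman encounter.
; When BP_Character overlaps its Trigger, it proceeds only if the UIInteract of the level's BP_Wife is hidden.
; It then hides its own UIInteract and, through a DoOnce, pauses the game, switches to UI-only input with a visible cursor and adds the dialogue widget to the viewport.
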(event OnComponentBeginOverlap(Trigger)
  (params (OverlappedComponent :type Primitive%20Component%20Object%20Reference) (OtherActor :type Actor%20Object%20Reference) (OtherComp :type Primitive%20Component%20Object%20Reference) (OtherBodyIndex :type Integer) (bFromSweep :type Boolean) (SweepResult :type Hit%20Result%20Structure%20%28by%20ref%29))
  (bind _returnvalue (Game|GetPlayerController 0))
  (Utilities|Casting|CastToBP_Character OtherActor)
  (bind _returnvalue_2 (Actor|GetActorOfClass "/Game/Blueprints/DeadBody/BP_Wife.BP_Wife_C"))
  (if (not (Rendering|IsVisible (Variables|/Game/Blueprints/DeadBody/BP_Wife.BP_Wife_C|GetUI_interact _returnvalue_2)))
    (Rendering|SetVisibility (Variables|Default|GetUI_Interact) false false)
    (Utilities|FlowControl|DoOnce false
      (:Completed
        (Game|SetGamePaused true)
        (Input|SetInputModeUIOnly _returnvalue 0 "DoNotLock" false)
        (Variables|/Script/Engine.PlayerController|SetbShowMouseCursor _returnvalue true)
        (bind _returnvalue_3 (UserInterface|CreateWidget "/Game/UIandWidget/FirstDialog/UI_DiaWife2.UI_DiaWife2_C"))
        (UserInterface|Viewport|AddtoViewport _returnvalue_3 0)))))

(event EventBeginPlay)

(event Collision|EventActorBeginOverlap
  (params (OtherActor :type Actor%20Object%20Reference)))

(event EventTick
  (params (DeltaSeconds :type Float%20%28single-precision%29)))

(fn ConstructionScript)