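; BP_Mystery2 is a mysterious-woman actor that opens the UI_DiaWife7 screen, apparently a dialogue, when BP_Character enters its Trigger.
; Overlap hides the UIInteract component, then a DoOnce runs the sequence a single time.
; It toggles the player's holster and removes the main UI held by BP_Instance.
; After a short delay it pauses the game, switches to UI-only input with a visible cursor and shows the widget.
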(event OnComponentBeginOverlap(Trigger)
  (params (OverlappedComponent :type Primitive%20Component%20Object%20Reference) (OtherActor :type Actor%20Object%20Reference) (OtherComp :type Primitive%20Component%20Object%20Reference) (OtherBodyIndex :type Integer) (bFromSweep :type Boolean) (SweepResult :type Hit%20Result%20Structure%20%28by%20ref%29))
  (bind _returnvalue (Game|GetPlayerController 0))
  (Utilities|Casting|CastToBP_Character OtherActor)
  (Rendering|SetVisibility (Variables|Default|GetUI_Interact) false false)
  (Utilities|FlowControl|DoOnce false
    (:Completed
      (bind _asbp_character (Utilities|Casting|CastToBP_Character (Game|GetPlayerCharacter 0)))
      (Default|HolsterToggle _asbp_character)
      (bind _asbp_instance (Utilities|Casting|CastToBP_Instance (Game|GetGameInstance)))
      (Widget|RemovefromParent (Variables|/Game/Blueprints/BP_Instance.BP_Instance_C|GetUI_main _asbp_instance))
      (Utilities|FlowControl|Delay 0.5)
      (Game|SetGamePaused true)
      (Input|SetInputModeUIOnly _returnvalue 0 "DoNotLock" false)
      (Variables|/Script/Engine.PlayerController|SetbShowMouseCursor _returnvalue true)
      (bind _returnvalue_2 (UserInterface|CreateWidget "/Game/UIandWidget/SecondDialog/UI_DiaWife7.UI_DiaWife7_C"))
      (UserInterface|Viewport|AddtoViewport _returnvalue_2 0))))

(event EventBeginPlay)

(event Collision|EventActorBeginOverlap
  (params (OtherActor :type Actor%20Object%20Reference)))

(event EventTick
  (params (DeltaSeconds :type Float%20%28single-precision%29)))

(fn ConstructionScript)