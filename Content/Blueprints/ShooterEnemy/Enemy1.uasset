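; Rifle-armed AI enemy that roams random reachable points, chases the player character on sight and shoots.
; SearchAround loops wandering via AIMoveTo; PawnSensing triggers ChaseTarget, which closes in, fires once and returns to searching.
; Fire faces the target, plays montage and effects, then applies damage through a debug-drawn line trace along the muzzle socket's up vector.
; At zero health, it ragdolls, disabling movement and capsule collision.
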(event OnSeePawn(PawnSensing)
  (params (Pawn :type Pawn%20Object%20Reference))
  (Utilities|Casting|CastToBP_Character Pawn)
  (CallFunction|ChaseTarget Pawn))

(event Custom|Search%20Around
  (if (not (Variables|Default|GetIsDead?))
    (AI|AIMoveTo self (.RandomLocation (AI|Navigation|GetRandomReachablePointinRadius (Transformation|GetActorLocation) 2e+04 0 0)) 0 1.2e+02 false
      (:OnSuccess
        (Utilities|FlowControl|Delay 1.0)
        (CallFunction|SearchAround)))))

(event Custom|Chase%20target
  (params (TargetActor :type Actor%20Object%20Reference))
  (if (not (Variables|Default|GetIsDead?))
    (AI|AIMoveTo self "0, 0, 0" TargetActor 5e+02 false
      (:OnSuccess
        (CallFunction|Fire TargetActor)
        (Utilities|FlowControl|Delay 1.0)
        (CallFunction|SearchAround))
      (:OnFail
        (CallFunction|SearchAround)))))

(event Custom|Fire
  (params (Target%20Actor :type Actor%20Object%20Reference))
  (bind _rifle (Variables|Default|GetRifle))
  (bind _returnvalue (Transformation|GetSocketTransform _rifle "b_gun_muzzleflash" "RTS_World"))
  (if (not (Variables|Default|GetIsDead?))
    (Pawn|SetControlRotation (Pawn|GetController) (Math|Rotator|FindLookatRotation (Transformation|GetActorLocation) (Transformation|GetActorLocation Target%20Actor)))
    (Animation|Montage|PlayMontage (Variables|Character|GetMesh) "/Game/Blueprints/ShooterEnemy/Fire_Rifle_Hip2_Montage.Fire_Rifle_Hip2_Montage"
      (:then
        (Effects|SpawnEmitterAttached "/Game/Realistic_Starter_VFX_Pack_Vol2/Particles/Explosion/P_Explosion_Big_A.P_Explosion_Big_A" (Variables|Default|GetRifle) "b_gun_muzzleflash" "0, 0, 0" "0, 0, 0" "0.030000,0.030000,0.030000")
        (Audio|PlaySoundatLocation "/Game/Audio/MSC_GunFire.MSC_GunFire" (Transformation|GetActorLocation) "0, 0, 0" 1.0 1.0 0.0 0 0 0 0)
        (bind (_outhit _returnvalue_2) (Collision|LineTraceByChannel (.location _returnvalue) (+ (.location _returnvalue) (* (Math|Vector|GetUpVector (.rotation _returnvalue)) 3e+03)) "TraceTypeQuery1" false 0 "ForDuration"))
        (if _returnvalue_2
          (Game|Damage|ApplyDamage (.HitActor (Collision|BreakHitResult _outhit)) 1e+01 0 0))))))

(event Game|Damage|EventAnyDamage
  (params (Damage :type Float%20%28single-precision%29) (DamageType :type Damage%20Type%20Object%20Reference) (InstigatedBy :type Controller%20Object%20Reference) (DamageCauser :type Actor%20Object%20Reference))
  (bind _output_get (Variables|Default|SetHealth (- (Variables|Default|GetHealth) Damage)))
  (if (<= _output_get 0.0)
    (Physics|SetSimulatePhysics (Variables|Character|GetMesh) true)
    (Variables|Default|SetIsDead? true)
    (Pawn|Components|CharacterMovement|SetMovementMode (Variables|Character|GetCharacterMovement) "MOVE_None" 0)
    (Collision|SetCollisionEnabled (Variables|Collision|GetCapsuleComponent) "NoCollision")))

(event EventBeginPlay
  (CallFunction|SearchAround))

(fn ConstructionScript)