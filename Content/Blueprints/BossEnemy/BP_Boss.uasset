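; Boss enemy character that chases the player once seen, attacks up close and dies when its health runs out.
; Pawn sensing starts a looping timer that moves it toward the player, sphere-tracing to apply damage on arrival.
; A separate loop replays the attack montage while the player is in range, independently of damage.
; Death ragdolls the mesh, disables capsule collision and movement, and plays a sound.
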(event OnSeePawn(PawnSensing)
  (params (Pawn :type Pawn%20Object%20Reference))
  (Variables|Default|SetIsSeeingPlayer? true)
  (CallFunction|UpdateChasing))

(event Custom|Follow%20Player
  (bind _attack_trace_point (Variables|Default|GetAttack%20Trace%20Point))
  (bind _returnvalue (Transformation|GetWorldLocation _attack_trace_point))
  (if (not (Variables|Default|GetDeath))
    (if (Variables|Default|GetIsSeeingPlayer?)
      (AI|AIMoveTo self "0, 0, 0" (Game|GetPlayerCharacter 0) 7e+01 false
        (:OnSuccess
          (bind (_outhit _returnvalue_2) (Collision|SphereTraceForObjects _returnvalue (+ _returnvalue (* (Math|Vector|GetForwardVector (Transformation|GetWorldRotation _attack_trace_point)) 7e+01)) 5e+01 (Utilities|Array|MakeArray "ObjectTypeQuery3") false 0 "None"))
          (if _returnvalue_2
            (bind _asbp_character (Utilities|Casting|CastToBP_Character (.HitActor (Collision|BreakHitResult _outhit))))
            (Game|Damage|ApplyDamage _asbp_character 2.0 0 0)))))))

(event Custom|Update%20Chasing
  (Utilities|Time|SetTimerbyEvent (delegate Custom|Follow%20Player) 0.1 true)
  (Utilities|FlowControl|Sequence
    (:then_0
      _)
    (:then_1
      _))
  (CallFunction|AttackCheckLoop))

(event Custom|Attack%20Check%20Loop
  (if (<= (Transformation|GetDistanceTo (Game|GetPlayerCharacter 0)) 1.5e+02) :!label _label
    (Utilities|FlowControl|Delay 0.1)
    (Variables|Default|SetCanAttack? false)
    (bind _returnvalue (Animation|PlayAnimMontage "/Game/Characters/Mannequins/Anims/Unarmed/Attack/MM_Attack_01_Montage.MM_Attack_01_Montage" 1.0 "None"))
    (Utilities|FlowControl|Delay _returnvalue)
    (Variables|Default|SetCanAttack? true)
    (goto _label)))

(event EventBeginPlay)

(event Collision|EventActorBeginOverlap
  (params (OtherActor :type Actor%20Object%20Reference)))

(event EventTick
  (params (DeltaSeconds :type Float%20%28single-precision%29)))

(event Game|Damage|EventAnyDamage
  (params (Damage :type Float%20%28single-precision%29) (DamageType :type Damage%20Type%20Object%20Reference) (InstigatedBy :type Controller%20Object%20Reference) (DamageCauser :type Actor%20Object%20Reference))
  (bind _output_get (Variables|Default|SetHealth (- (Variables|Default|GetHealth) Damage)))
  (if (<= _output_get 0.0)
    (Physics|SetSimulatePhysics (Variables|Character|GetMesh) true)
    (Pawn|Components|CharacterMovement|SetMovementMode (Variables|Character|GetCharacterMovement) "MOVE_None" 0)
    (Audio|PlaySoundatLocation "/Game/Audio/492492__soundflakes__demon-death-01.492492__soundflakes__demon-death-01" (Transformation|GetActorLocation) "0, 0, 0" 1.0 1.0 0.0 0 0 0 0)
    (Collision|SetCollisionEnabled (Variables|Collision|GetCapsuleComponent) "NoCollision")
    (Variables|Default|SetDeath true)))

(fn ConstructionScript)